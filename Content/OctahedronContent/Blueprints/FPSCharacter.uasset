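; First-person character Blueprint handling look, move, jump, crouch and firing of a rifle spawned as a child actor.
; A timeline blends capsule height and walk speed for crouch; on release, a looping sphere trace waits for headroom before reversing it.
; A speed-scaled coyote timer extends the jump window, and jumps and landings trigger a timeline camera-style dip of Root.
; Walk-bob and velocity-lag calculations exist, but their timeline is never started here.
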(event Input|EnhancedActionEvents|EnhancedInputActionIA_Look
  (params (ActionValue :type Vector%202D%20Structure) (ElapsedSeconds :type Float%20%28double-precision%29) (TriggeredSeconds :type Float%20%28double-precision%29) (InputAction :type Input%20Action%20Object%20Reference :default "/Game/FPSDefaultContent/FirstPerson/Input/Actions/IA_Look.IA_Look"))
  (Pawn|Input|AddControllerYawInput (.x ActionValue))
  (Pawn|Input|AddControllerPitchInput (.y ActionValue)))

(event Input|EnhancedActionEvents|EnhancedInputActionIA_Move
  (params (ActionValue :type Vector%202D%20Structure) (ElapsedSeconds :type Float%20%28double-precision%29) (TriggeredSeconds :type Float%20%28double-precision%29) (InputAction :type Input%20Action%20Object%20Reference :default "/Game/FPSDefaultContent/FirstPerson/Input/Actions/IA_Move.IA_Move"))
  (Pawn|Input|AddMovementInput (Transformation|GetActorRightVector) (.x ActionValue) false)
  (Pawn|Input|AddMovementInput (Transformation|GetActorForwardVector) (.y ActionValue) false))

(event Input|EnhancedActionEvents|EnhancedInputActionIA_Jump
  (params (ActionValue :type Boolean) (ElapsedSeconds :type Float%20%28double-precision%29) (TriggeredSeconds :type Float%20%28double-precision%29) (InputAction :type Input%20Action%20Object%20Reference :default "/Game/FPSDefaultContent/FirstPerson/Input/Actions/IA_Jump.IA_Jump"))
  (:Started
    (Character|Jump))
  (:Completed
    (Character|StopJumping)))

(event Input|EnhancedActionEvents|EnhancedInputActionIA_Shoot
  (params (ActionValue :type Boolean) (ElapsedSeconds :type Float%20%28double-precision%29) (TriggeredSeconds :type Float%20%28double-precision%29) (InputAction :type Input%20Action%20Object%20Reference :default "/Game/FPSDefaultContent/FirstPerson/Input/Actions/IA_Shoot.IA_Shoot"))
  (Default|Fire (CallFunction|GetWeapon)))

(event Custom|Standup
  (bind _crouchalpha (Timeline|StandupLine Reverse)
    (:Update
      (Variables|crouch|SetcrouchAlpha _crouchalpha)
      (Variables|/Script/Engine.CharacterMovementComponent|SetMaxWalkSpeed (Variables|Character|GetCharacterMovement) (Math|Float|Lerp (Variables|Default|GetwalkSpeed) (Variables|crouch|GetcrouchSpeed) (Variables|crouch|GetcrouchAlpha)))
      (Components|Capsule|SetCapsuleHalfHeight (Variables|Collision|GetCapsuleComponent) (Math|Float|Lerp (Variables|Default|GetstandHeight) (Variables|crouch|GetcrouchHeight) (Variables|crouch|GetcrouchAlpha)) true))))

(event Custom|CoyoteTimePassed)

(event Custom|Dip
  (params (speed :type Float%20%28double-precision%29) (strength :type Float%20%28double-precision%29))
  (bind _root (Variables|Default|GetRoot))
  (bind _relativelocation (Variables|/Script/Engine.SceneComponent|GetRelativeLocation _root))
  (bind (_x _y) (Math|Vector|BreakVector _relativelocation))
  (Components|Timeline|SetPlayRate (Variables|Default|GetDipLine) speed)
  (Variables|Default|SetdipStrength strength)
  (bind _dipalpha (Timeline|DipLine PlayFromStart)
    (:Update
      (bind _output_get (Variables|Default|SetdipAlpha (* _dipalpha (Variables|Default|GetdipStrength))))
      (Transformation|SetRelativeLocation _root (Math|Vector|MakeVector _x _y (Math|Float|Lerp 0.0 -1e+01 _output_get)) false false))))

(event Custom|LandingDip
  (bind _charactermovement (Variables|Character|GetCharacterMovement))
  (CallFunction|Dip 3.0 (Math|Float|Clamp(Float) (Math|Float|NormalizetoRange (Math|Vector|VectorLength (Math|Vector|MakeVector 0.0 0.0 (.Z (Math|Vector|BreakVector (Pawn|Components|CharacterMovement|GetLastUpdateVelocity _charactermovement))))) 0.0 (Variables|/Script/Engine.CharacterMovementComponent|GetJumpZVelocity _charactermovement)))))

(event Input|EnhancedActionEvents|EnhancedInputActionIA_Crouch
  (params (ActionValue :type Boolean) (ElapsedSeconds :type Float%20%28double-precision%29) (TriggeredSeconds :type Float%20%28double-precision%29) (InputAction :type Input%20Action%20Object%20Reference :default "/Game/FPSDefaultContent/FirstPerson/Input/Actions/IA_Crouch.IA_Crouch"))
  (:Started
    (Utilities|Time|ClearandInvalidateTimerbyHandle (Variables|Default|GetcheckCanStandTimer))
    (bind _crouchalpha (Timeline|StandupLine Play)
      (:Update
        (Variables|crouch|SetcrouchAlpha _crouchalpha)
        (Variables|/Script/Engine.CharacterMovementComponent|SetMaxWalkSpeed (Variables|Character|GetCharacterMovement) (Math|Float|Lerp (Variables|Default|GetwalkSpeed) (Variables|crouch|GetcrouchSpeed) (Variables|crouch|GetcrouchAlpha)))
        (Components|Capsule|SetCapsuleHalfHeight (Variables|Collision|GetCapsuleComponent) (Math|Float|Lerp (Variables|Default|GetstandHeight) (Variables|crouch|GetcrouchHeight) (Variables|crouch|GetcrouchAlpha)) true))))
  (:Completed
    (bind _returnvalue (Utilities|Time|SetTimerbyFunctionName 0 "CheckCanStand" 0.016667 true))
    (Variables|Default|SetcheckCanStandTimer _returnvalue)))

(event EventOnMovementModeChanged
  (params (PrevMovementMode :type EMovementMode%20Enum :default "MOVE_None") (NewMovementMode :type EMovementMode%20Enum :default "MOVE_None") (PrevCustomMode :type Byte :default 0) (NewCustomMode :type Byte :default 0))
  (if (Utilities|Enum|Equal(Enum) NewMovementMode "MOVE_Falling")
    (bind _returnvalue (Utilities|Time|SetTimerbyEvent (delegate Custom|CoyoteTimePassed) (* (Math|Float|Lerp 0.25 1.0 (Math|Float|Clamp(Float) (Math|Float|NormalizetoRange (Math|Vector|VectorLength (Transformation|GetVelocity)) 0.0 (Variables|Default|GetwalkSpeed)))) (Variables|Default|GetcoyoteTime))))
    (Variables|Default|SetcoyoteTimer _returnvalue)))

(event EventOnLanded
  (params (Hit :type Hit%20Result%20Structure%20%28by%20ref%29))
  (CallFunction|LandingDip)
  (Utilities|Time|ClearandInvalidateTimerbyHandle (Variables|Default|GetcoyoteTimer)))

(event EventOnJumped
  (CallFunction|Dip 5.0 1.0)
  (Utilities|Time|ClearandInvalidateTimerbyHandle (Variables|Default|GetcoyoteTimer)))

(fn ConstructionScript
  (bind _charactermovement (Variables|Character|GetCharacterMovement))
  (ChildActorComponent|SetChildActorClass (Variables|Default|GetWeapon) "/Game/OctahedronContent/Blueprints/RifleWeapon.RifleWeapon_C")
  (Variables|Default|SetwalkSpeed (Variables|/Script/Engine.CharacterMovementComponent|GetMaxWalkSpeed _charactermovement))
  (Variables|crouch|SetcrouchSpeed (Variables|/Script/Engine.CharacterMovementComponent|GetMaxWalkSpeedCrouched _charactermovement))
  (Variables|crouch|SetcrouchHeight (Variables|/Script/Engine.CharacterMovementComponent|GetCrouchedHalfHeight _charactermovement))
  (Variables|Default|SetstandHeight (Variables|/Script/Engine.CapsuleComponent|GetCapsuleHalfHeight (Variables|Collision|GetCapsuleComponent))))

(fn GetWeapon
  (bind _asweapon_base (Utilities|Casting|CastToWeaponBase (Variables|/Script/Engine.ChildActorComponent|GetChildActor (Variables|Default|GetWeapon)))
    (:then
      (return _asweapon_base))
    (:CastFailed
      (Development|PrintString "Cast to weapon fails!"))))

(fn CheckCanStand
  (bind _returnvalue (Transformation|GetActorLocation))
  (bind _crouchheight (Variables|crouch|GetcrouchHeight))
  (bind (_x _y _z) (Math|Vector|BreakVector _returnvalue))
  (bind _returnvalue_2 (+ _z _crouchheight))
  (bind _returnvalue_3 (Collision|SphereTraceByChannel (Math|Vector|MakeVector _x _y _returnvalue_2) (Math|Vector|MakeVector _x _y (+ _returnvalue_2 (* (Math|Float|Lerp 0.0 (- (Variables|Default|GetstandHeight) _crouchheight) (Variables|crouch|GetcrouchAlpha)) 1.1))) (* (Variables|/Script/Engine.CapsuleComponent|GetCapsuleRadius (Variables|Collision|GetCapsuleComponent)) 0.5) "TraceTypeQuery1" false (Utilities|Array|MakeArray self) "None"))
  (if (or (not _returnvalue_3) (AI|Components|NavMovement|IsFalling (Variables|Character|GetCharacterMovement)))
    (CallFunction|Standup)
    (Utilities|Time|ClearandInvalidateTimerbyHandle (Variables|Default|GetcheckCanStandTimer))))

(fn CanJumpInternal
  (bind _returnvalue (|CallParentFunction))
  (return (and (or _returnvalue (> (Utilities|Time|GetTimerRemainingTimebyHandle (Variables|Default|GetcoyoteTimer)) 0.0)) (not (Utilities|Time|IsTimerActivebyHandle (Variables|Default|GetcheckCanStandTimer))))))

(fn CalcVelocityVars
  (bind _returnvalue (Transformation|GetVelocity))
  (bind _returnvalue_2 (Utilities|Time|GetWorldDeltaSeconds))
  (bind _walkspeed (Variables|Default|GetwalkSpeed))
  (Variables|Default|SetlagPos (Math|Interpolation|VInterpTo (Variables|Default|GetlagPos) (Math|Vector|ClampVectorSize (* (Math|Vector|MakeVector (/ (Math|Vector|DotProduct _returnvalue (Transformation|GetActorRightVector)) _walkspeed) (/ (Math|Vector|DotProduct _returnvalue (Transformation|GetActorForwardVector)) (* _walkspeed -1.0)) (/ (Math|Vector|DotProduct _returnvalue (Transformation|GetActorUpVector)) (* (Variables|/Script/Engine.CharacterMovementComponent|GetJumpZVelocity (Variables|Character|GetCharacterMovement)) -1.0))) 2.0) 0.0 4.0) _returnvalue_2 (/ 0.166667 _returnvalue_2))))