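; WeaponBase is a base weapon for the FPS character, with empty Equip, Stow, Fire and Reload events.
; On BeginPlay it caches its parent character and adds the weapons input mapping context, while construction applies the configured mesh and material.
; Hitscan traces from the camera within a random spread cone and stores that hit, then traces from the muzzle toward that point, with optional debug drawing.
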(event Custom|Fire)

(event Custom|Equip)

(event Custom|Stow)

(event Custom|Reload)

(event EventBeginPlay
  (bind _asfpscharacter (Utilities|Casting|CastToFPSCharacter (Actor|GetParentActor)))
  (bind _output_get (Variables|Default|Setplayer _asfpscharacter))
  (bind _asplayer_controller (Utilities|Casting|CastToPlayerController (Pawn|GetController _output_get)))
  (Utilities|IsValid (PlayerController|LocalPlayerSubsystems|GetEnhancedInputLocalPlayerSubsystem _asplayer_controller)
    (:Is%20Valid
      (Input|AddMappingContext (PlayerController|LocalPlayerSubsystems|GetEnhancedInputLocalPlayerSubsystem _asplayer_controller) "/Game/FPSDefaultContent/FirstPerson/Input/IMC_Weapons.IMC_Weapons" 0 "(bIgnoreAllPressedKeysUntilRelease=True,bForceImmediately=False,bNotifyUserSettings=False)"))))

(fn ConstructionScript
  (bind _skeletalmesh (Variables|Default|GetSkeletalMesh))
  (Components|SkeletalMesh|SetSkeletalMeshAsset _skeletalmesh (Variables|Default|GetweaponMesh))
  (Rendering|Material|SetMaterial _skeletalmesh 0 (Variables|Default|GetweaponMaterial)))

(fn Hitscan
  (params (drawDebug :type Boolean))
  (bind _player (Variables|Default|Getplayer))
  (bind _spread (Variables|Default|Getspread))
  (bind _camera (Variables|/Game/OctahedronContent/Blueprints/FPSCharacter.FPSCharacter_C|GetCamera _player))
  (bind _returnvalue (Math|Vector|GetForwardVector _camera))
  (bind _returnvalue_2 (Transformation|GetWorldLocation _camera))
  (bind _returnvalue_3 (Math|Random|RandomUnitVectorinConeinDegrees _returnvalue _spread))
  (bind (_outhit _returnvalue_4) (Collision|LineTraceByChannel _returnvalue_2 (+ _returnvalue_2 (* _returnvalue_3 (Variables|Default|Getrange))) "TraceTypeQuery1" false (Utilities|Array|MakeArray (Variables|Default|Getplayer)) (select drawDebug "ForDuration" "None")))
  (LocalVariables|SethitInfo _outhit)
  (Collision|LineTraceByChannel (Transformation|GetSocketLocation (Variables|Default|GetSkeletalMesh) "Muzzle") (Math|Vector|SelectVector (+ (.Location (Collision|BreakHitResult _outhit)) (* _returnvalue_3 1e+01)) (.TraceEnd (Collision|BreakHitResult _outhit)) _returnvalue_4) "TraceTypeQuery1" false (Utilities|Array|MakeArray (Variables|Default|Getplayer)) (select drawDebug "ForDuration" "None") true "(R=1.000000,G=1.000000,B=0.000000,A=1.000000)" "(R=0.000000,G=0.000000,B=1.000000,A=1.000000)"))